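; Cupcake pickup, a child Blueprint of a parent pickup, that adds coins through the game mode when collected.
; On BeginPlay it runs the parent logic, then binds its own event to the parent's On Picked Up dispatcher.
; That event casts the game mode to ThirdPersonGameMode and calls its coin-adding function.
; An unconnected super jump snippet that raises the player's jump velocity and prints a message never runs.
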(event `self.ReceiveBeginPlay`
  (`parent.ReceiveBeginPlay`) ; This fires off the "ReceiveBeginPlay" event in the parent script
  (add `self.On Picked up` (delegate `Pickup grabbed`)) ; Bind the "Pickup grabbed" custom event to the function "On Picked up", which is called in the parent Blueprint script
)

(event `Pickup grabbed`
  (bind _asthird_person_game_mode (cast `/Game/ThirdPersonBP/Blueprints/ThirdPersonGameMode` (`GameplayStatics.GetGameMode`)))
  (`/Game/ThirdPersonBP/Blueprints/ThirdPersonGameMode.addcoins11` _asthird_person_game_mode))

(fn `UserConstructionScript`
  (`parent.UserConstructionScript`))