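; Coin pickup child Blueprint that triggers a coin-adding call when the player collects it.
; On BeginPlay it runs the parent logic and binds its grabbed event to the parent's On Picked Up dispatcher.
; That event attempts a Game Mode cast with no visible target class, then calls the add-coins function.
; A disconnected max walk speed change and an empty extra function are unused leftovers.
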(event `self.ReceiveBeginPlay`
  (`parent.ReceiveBeginPlay`) ; This fires off the "ReceiveBeginPlay" event in the parent script
  (add `self.On Picked up` (delegate `Pickup grabbed`)) ; Bind the "Pickup grabbed" custom event to the function "On Picked up", which is called in the parent Blueprint script
)

(event `Pickup grabbed`
  (cast `` (`GameplayStatics.GetGameMode`)
    (:`then`
      _)
    (:`CastFailed`
      _))
  (`/Game/ThirdPersonBP/Blueprints/ThirdPersonGameMode.addcoins11`))

(fn `NewFunction_0`)

(fn `UserConstructionScript`
  (`parent.UserConstructionScript`))